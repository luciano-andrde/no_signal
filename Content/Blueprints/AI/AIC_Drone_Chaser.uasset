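; AI controller for the chaser enemy drone that drives it straight at a target pawn.
; On possess it caches the controlled drone, and a SetTargetPlayer event supplies the target.
; Each tick, while both are valid, it turns the look-at rotation into a direction vector for the drone's MoveTowards at full scale, with no pathfinding or behavior tree.
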(event Custom|Set%20Target%20Player
  (params (target_pawn :type Pawn%20Object%20Reference))
  (Variables|Default|Settarget_pawn target_pawn))

(event EventTick
  (params (DeltaSeconds :type Float%20%28single-precision%29))
  (|CallParentFunction DeltaSeconds)
  (Utilities|IsValid (Variables|Default|Getowning_drone_chaser)
    (:Is%20Valid
      (Utilities|IsValid (Variables|Default|Gettarget_pawn)
        (:Is%20Valid
          (Default|MoveTowards (Variables|Default|Getowning_drone_chaser) (Math|Vector|GetForwardVector (Math|Rotator|FindLookatRotation (Transformation|GetActorLocation (Variables|Default|Getowning_drone_chaser)) (Transformation|GetActorLocation (Variables|Default|Gettarget_pawn)))) 1.0))))))

(event EventPossess
  (params (PossessedPawn :type Pawn%20Object%20Reference))
  (bind _asbp_enemy_drone_chaser (Utilities|Casting|CastToBP_Enemy_Drone_Chaser PossessedPawn))
  (Variables|Default|Setowning_drone_chaser _asbp_enemy_drone_chaser))

(fn ConstructionScript
  (|CallParentFunction))