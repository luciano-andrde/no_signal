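; BP_Action_Character_BASE is a base action character that handles damage, defeat and sprite hit feedback.
; Incoming damage goes to the BPCVitality component, which decides whether the actor is destroyed or flashes red.
; The flash drives color and multiplier parameters on a dynamic sprite material created at BeginPlay, with a rate-adjustable timeline fading the multiplier to zero.
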(event Custom|TriggerFlash
  (params (Flash%20Multiplier :type Float%20%28single-precision%29) (Flash%20Color :type Linear%20Color%20Structure))
  (Rendering|Material|SetScalarParameterValue (Variables|Default|Getdynamic_sprite_material) "Flash Multiplier" Flash%20Multiplier :!class /Script/Engine.MaterialInstanceDynamic)
  (Rendering|Material|SetVectorParameterValue (Variables|Default|Getdynamic_sprite_material) "Flash Color" Flash%20Color :!class /Script/Engine.MaterialInstanceDynamic)
  (Components|Timeline|SetPlayRate (Variables|Default|GetFade%20Sprite%20Flash) (Variables|Default|Getsprite_flash_play_rate))
  (bind _alpha (Timeline|Fade%20Sprite%20Flash PlayFromStart)
    (:Update
      (Rendering|Material|SetScalarParameterValue (Variables|Default|Getdynamic_sprite_material) "Flash Multiplier" (Math|Float|Lerp Flash%20Multiplier 0.0 _alpha) :!class /Script/Engine.MaterialInstanceDynamic))))

(event Collision|EventActorBeginOverlap
  (params (OtherActor :type Actor%20Object%20Reference)))

(event EventTick
  (params (DeltaSeconds :type Float%20%28single-precision%29)))

(event Game|Damage|EventAnyDamage
  (params (Damage :type Float%20%28single-precision%29) (DamageType :type Damage%20Type%20Object%20Reference) (InstigatedBy :type Controller%20Object%20Reference) (DamageCauser :type Actor%20Object%20Reference))
  (Default|ReceiveDamage (Variables|Default|GetBPC_Vitality) Damage)
  (if (Variables|/Game/Blueprints/Components/BPC_Vitality.BPC_Vitality_C|Getis_defeated (Variables|Default|GetBPC_Vitality))
    (Actor|DestroyActor)
    (else
      (CallFunction|TriggerFlash 4e+01 "(R=1.000000,G=0.026042,B=0.026042,A=1.000000)"))))

(event EventBeginPlay
  (bind _returnvalue (Rendering|Material|CreateDynamicMaterialInstance (Variables|Default|GetSprite) 0 0 "None" :!class /Script/Engine.PrimitiveComponent))
  (Variables|Default|Setdynamic_sprite_material _returnvalue))

(fn ConstructionScript)