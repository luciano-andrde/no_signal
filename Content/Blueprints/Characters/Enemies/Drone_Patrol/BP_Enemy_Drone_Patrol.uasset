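; Patrol drone enemy that shuttles back and forth between two points marked by its TopPosition and BottomPosition components.
; BeginPlay caches both world positions, so the endpoints stay fixed as the actor moves, then starts the MoveAnim timeline at a configurable play rate.
; The timeline lerps actor location without sweep, and a FlipFlop on Finished alternates reverse and forward playback for an endless loop.
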(event Custom|Move%20Forward
  (bind _alpha (Timeline|MoveAnim PlayFromStart)
    (:Update
      (Transformation|SetActorLocation (Math|Vector|Lerp(Vector) (Variables|Default|GetWorld%20Top%20Position) (Variables|Default|GetWorld%20Bottom%20Position) _alpha) false false))
    (:Finished
      (Utilities|FlowControl|FlipFlop
        (:A
          (CallFunction|MoveBackward))
        (:B
          (CallFunction|MoveForward))))))

(event Custom|Move%20Backward
  (bind _alpha (Timeline|MoveAnim ReverseFromEnd)
    (:Update
      (Transformation|SetActorLocation (Math|Vector|Lerp(Vector) (Variables|Default|GetWorld%20Top%20Position) (Variables|Default|GetWorld%20Bottom%20Position) _alpha) false false))
    (:Finished
      (Utilities|FlowControl|FlipFlop
        (:A
          (CallFunction|MoveBackward))
        (:B
          (CallFunction|MoveForward))))))

(event EventBeginPlay
  (|CallParentFunction)
  (Variables|Default|SetWorld%20Top%20Position (Transformation|GetWorldLocation (Variables|Default|GetTop%20Position)))
  (Variables|Default|SetWorld%20Bottom%20Position (Transformation|GetWorldLocation (Variables|Default|GetBottom%20Position)))
  (Components|Timeline|SetPlayRate (Variables|Default|GetMoveAnim) (Variables|Default|Getmove_play_rate))
  (CallFunction|MoveForward))

(event Collision|EventActorBeginOverlap
  (params (OtherActor :type Actor%20Object%20Reference))
  (|CallParentFunction OtherActor) ; This node is disabled and will not be called.\nDrag off pins to build functionality.
)

(event EventTick
  (params (DeltaSeconds :type Float%20%28single-precision%29))
  (|CallParentFunction DeltaSeconds) ; This node is disabled and will not be called.\nDrag off pins to build functionality.
)

(fn ConstructionScript
  (|CallParentFunction))