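; Static drone enemy Blueprint that fires fireball projectiles.
; Shoot Fireball plays the Fire sequence as an animation override on the animation component's instance.
; A separate Spawn Fireball function always spawns a static drone projectile at the ShootPosition component's world location and rotation, regardless of collision.
; Neither function is called within this Blueprint, and its event graph holds only disabled default events.
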(event EventBeginPlay
  (|CallParentFunction) ; This node is disabled and will not be called.\nDrag off pins to build functionality.
)

(event Collision|EventActorBeginOverlap
  (params (OtherActor :type Actor%20Object%20Reference))
  (|CallParentFunction OtherActor) ; This node is disabled and will not be called.\nDrag off pins to build functionality.
)

(event EventTick
  (params (DeltaSeconds :type Float%20%28single-precision%29))
  (|CallParentFunction DeltaSeconds) ; This node is disabled and will not be called.\nDrag off pins to build functionality.
)

(fn ConstructionScript
  (|CallParentFunction))

(fn ShootFireball
  (Class|PaperZDAnimInstance|PlayAnimationOverride (Variables|/Script/PaperZD.PaperZDAnimationComponent|GetAnimInstance (Variables|Default|GetAnimationComponent)) "/Game/Blueprints/Characters/Enemies/Static_Drone/AnimSequences/Fire.Fire" "DefaultSlot" 1.0 0.0))

(fn SpawnFireball
  (bind _shoot_position (Variables|Default|GetShoot%20Position))
  (Game|SpawnActorfromClass "/Game/Blueprints/Projectiles/Enemy/BP_Enemy_Projectile_Static_Drone.BP_Enemy_Projectile_Static_Drone_C" (Math|Transform|MakeTransform (Transformation|GetWorldLocation _shoot_position) (Transformation|GetWorldRotation _shoot_position) "1.000000,1.000000,1.000000") "AlwaysSpawn" "MultiplyWithRoot" 0 0))