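; BPC_Vitality is a Blueprint component that tracks health and defeat state.
; BeginPlay fills current health to the maximum.
; ReceiveDamage subtracts damage, clamps the result between zero and the maximum, then either sets the IsDefeated flag at zero or prints the remaining health.
; It only sets the flag on defeat, with no event broadcast or further reaction.
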(event EventBeginPlay
  (Variables|Default|Setcurrent_health (Variables|Default|Getmax_health)))

(event EventTick
  (params (DeltaSeconds :type Float%20%28single-precision%29)))

(fn ReceiveDamage
  (params (Damage :type Float%20%28double-precision%29))
  (Variables|Default|Setcurrent_health (Math|Float|Clamp(Float) (- (Variables|Default|Getcurrent_health) Damage) 0.0 (Variables|Default|Getmax_health)))
  (if (<= (Variables|Default|Getcurrent_health) 0.0)
    (Variables|Default|Setis_defeated true)
    (else
      (Development|PrintString (Utilities|String|ToString(Float) (Variables|Default|Getcurrent_health))))))