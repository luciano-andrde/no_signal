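; Game mode that handles player respawning with checkpoint support.
; On BeginPlay it caches a PlayerStart found in the level as the fallback spawn point.
; RespawnPlayer spawns the default pawn at the active checkpoint's Scene component, or at that PlayerStart when no checkpoint is valid, ignoring collisions, then has player controller 0 possess it.
; The active checkpoint is only read here, and the previous pawn is not destroyed.
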(event EventBeginPlay
  (bind _returnvalue (Actor|GetActorOfClass "/Script/Engine.PlayerStart"))
  (Variables|Default|Setplayer_start _returnvalue))

(event EventTick
  (params (DeltaSeconds :type Float%20%28single-precision%29)))

(fn ConstructionScript)

(fn RespawnPlayer
  (bind _player_start (Variables|Default|Getplayer_start))
  (bind _active_checkpoint (Variables|Default|Getactive_checkpoint))
  (bind _returnvalue (Transformation|GetActorTransform _player_start))
  (bind _scene (Variables|/Game/Blueprints/Props/BP_Checkpoint.BP_Checkpoint_C|GetScene _active_checkpoint))
  (bind _returnvalue_2 (Transformation|GetWorldTransform _scene))
  (Utilities|IsValid (Variables|Default|Getactive_checkpoint)
    (:Is%20Valid
      (bind _returnvalue_3 (Game|SpawnActorfromClass (Variables|Default|GetDefaultPawnClass) (Math|Transform|MakeTransform (.location _returnvalue_2) (.rotation _returnvalue_2) "1.000000,1.000000,1.000000") "AlwaysSpawn" "MultiplyWithRoot" 0 0))
      (Pawn|Possess (Game|GetPlayerController 0) _returnvalue_3))
    (:Is%20Not%20Valid
      (bind _returnvalue_4 (Game|SpawnActorfromClass (Variables|Default|GetDefaultPawnClass) (Math|Transform|MakeTransform (.location _returnvalue) (.rotation _returnvalue) "1.000000,1.000000,1.000000") "AlwaysSpawn" "MultiplyWithRoot" 0 0))
      (Pawn|Possess (Game|GetPlayerController 0) _returnvalue_4))))