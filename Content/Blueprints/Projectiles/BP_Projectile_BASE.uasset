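; BP_Projectile_BASE is a base projectile that kills action characters of an opposing faction.
; On sphere overlap with a BP_Action_Character_BASE whose Faction differs from its own, it destroys that character outright, with no damage step.
; A blocking hit or enemy kill spawns BP_VFX_Shoot_Hit at the projectile's transform and destroys the projectile.
; Overlaps with same-faction characters or other actor types are ignored.
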(event OnComponentHit(Sphere)
  (params (HitComponent :type Primitive%20Component%20Object%20Reference) (OtherActor :type Actor%20Object%20Reference) (OtherComp :type Primitive%20Component%20Object%20Reference) (NormalImpulse :type Vector :default "0, 0, 0") (Hit :type Hit%20Result%20Structure%20%28by%20ref%29))
  (CallFunction|PlayHitEffects)
  (Actor|DestroyActor))

(event OnComponentBeginOverlap(Sphere)
  (params (OverlappedComponent :type Primitive%20Component%20Object%20Reference) (OtherActor :type Actor%20Object%20Reference) (OtherComp :type Primitive%20Component%20Object%20Reference) (OtherBodyIndex :type Integer) (bFromSweep :type Boolean) (SweepResult :type Hit%20Result%20Structure%20%28by%20ref%29))
  (bind _asbp_action_character_base (Utilities|Casting|CastToBP_Action_Character_BASE OtherActor))
  (if (Utilities|Enum|NotEqual(Enum) (Variables|/Game/Blueprints/Characters/BP_Action_Character_BASE.BP_Action_Character_BASE_C|Getfaction _asbp_action_character_base) (Variables|Default|Getfaction))
    (Actor|DestroyActor _asbp_action_character_base)
    (CallFunction|PlayHitEffects)
    (Actor|DestroyActor)))

(event EventBeginPlay)

(event Collision|EventActorBeginOverlap
  (params (OtherActor :type Actor%20Object%20Reference)))

(event EventTick
  (params (DeltaSeconds :type Float%20%28single-precision%29)))

(fn ConstructionScript)

(fn PlayHitEffects
  (Game|SpawnActorfromClass "/Game/Blueprints/VFX/BP_VFX_Shoot_Hit.BP_VFX_Shoot_Hit_C" (Math|Transform|MakeTransform (Transformation|GetActorLocation) (Transformation|GetActorRotation) "1.000000,1.000000,1.000000") "AlwaysSpawn" "MultiplyWithRoot" 0 0))